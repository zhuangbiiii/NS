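; BP_Character is a player-controlled character that moves, looks, jumps and casts fireballs.
; Input axes drive movement along the actor's forward and right vectors and feed yaw and pitch to the controller, while the Jump action starts and stops jumping.
; The Skill action spawns BP_FireBall at the SpawnPoint component's location, aimed along the control rotation, with the character as Instigator.
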(event `InputAction|Skill`
  (params (Key :type "Key Structure"))
  (:`Pressed`
    (`|SpawnActorFromClass` "/Game/Blueprint/BP_FireBall.BP_FireBall_C" (`KismetMathLibrary.MakeTransform` (`SceneComponent.K2_GetComponentLocation` (`self.SpawnPoint`)) (`self.GetControlRotation`)) "Undefined" "OverrideRootScale" null self)))

(event `InputAction|Jump`
  (params (Key :type "Key Structure"))
  ;[1 1 1] 注释
  (:`Pressed`
    (`self.Jump`))
  (:`Released`
    (`self.StopJumping`)))

(event `InputAxis|MoveForward` :overrideparent false
  (params (AxisValue :type "Float (single-precision)"))
  ;[1 1 1] 注释
  (`self.AddMovementInput` (`self.GetActorForwardVector`) AxisValue))

(event `InputAxis|MoveRight` :overrideparent false
  (params (AxisValue :type "Float (single-precision)"))
  ;[1 1 1] 注释
  (`self.AddMovementInput` (`self.GetActorRightVector`) AxisValue))

(event `InputAxis|Turn` :overrideparent false
  (params (AxisValue :type "Float (single-precision)"))
  ;[1 1 1] 注释
  (`self.AddControllerYawInput` AxisValue))

(event `InputAxis|LookUp` :overrideparent false
  (params (AxisValue :type "Float (single-precision)"))
  ;[1 1 1] 注释
  (`self.AddControllerPitchInput` AxisValue))

(fn `UserConstructionScript`)